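; Track generator that lays out yellow and blue boundary cones from the Track data table in its Construction Script.
; Each row's yellow and blue XY pairs are scaled by Spacing as world coordinates, skipping zero entries.
; A vertical Visibility trace drops each point onto the surface, where a cone is added as a child actor offset from the root's location.
; Cones are tagged CY or CB plus a per-colour running index.
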(event EventBeginPlay)

(event Collision|EventActorBeginOverlap
  (params (OtherActor :type Actor%20Object%20Reference)))

(event EventTick
  (params (DeltaSeconds :type Float%20%28single-precision%29)))

(fn ConstructionScript
  (bind _track (Variables|Default|GetTrack))
  (bind _spacing (Variables|Default|GetSpacing))
  (Variables|Default|SetBlueCount 0)
  (Variables|Default|SetYellowCount 0)
  (bind _outrownames (DataTable|GetDataTableRowNames _track))
  (for _array_element _outrownames
    (bind _returnvalue (Utilities|GetDataTableRow _track _array_element)
      (:then
        (Utilities|FlowControl|Sequence
          (:then_0
            (if (Math|Vector|NotEqual(Vector) (* (Math|Vector|MakeVector (.Yellow_X (Utilities|Struct|BreakDS_Cones _returnvalue)) (.Yellow_y (Utilities|Struct|BreakDS_Cones _returnvalue)) 0.0) _spacing) "0, 0, 0" 0.0001)
              (bind _outhit (Collision|LineTraceByChannel (Math|Vector|MakeVector (.X (Math|Vector|BreakVector (* (Math|Vector|MakeVector (.Yellow_X (Utilities|Struct|BreakDS_Cones _returnvalue)) (.Yellow_y (Utilities|Struct|BreakDS_Cones _returnvalue)) 0.0) _spacing))) (.Y (Math|Vector|BreakVector (* (Math|Vector|MakeVector (.Yellow_X (Utilities|Struct|BreakDS_Cones _returnvalue)) (.Yellow_y (Utilities|Struct|BreakDS_Cones _returnvalue)) 0.0) _spacing))) 1e+03) (Math|Vector|MakeVector (.X (Math|Vector|BreakVector (* (Math|Vector|MakeVector (.Yellow_X (Utilities|Struct|BreakDS_Cones _returnvalue)) (.Yellow_y (Utilities|Struct|BreakDS_Cones _returnvalue)) 0.0) _spacing))) (.Y (Math|Vector|BreakVector (* (Math|Vector|MakeVector (.Yellow_X (Utilities|Struct|BreakDS_Cones _returnvalue)) (.Yellow_y (Utilities|Struct|BreakDS_Cones _returnvalue)) 0.0) _spacing))) -1e+03) "TraceTypeQuery1" false 0 "None"))
              (bind _returnvalue_2 (AddComponent|AddChildActorComponent false (Math|Transform|MakeTransform (- (.ImpactPoint (Collision|BreakHitResult _outhit)) (Transformation|GetWorldLocation (Variables|Default|GetDefaultSceneRoot))))))
              (ChildActorComponent|SetChildActorClass _returnvalue_2 (Variables|Default|GetYellowCone))
              (Variables|/Script/Engine.Actor|SetTags (Variables|/Script/Engine.ChildActorComponent|GetChildActor _returnvalue_2) (Utilities|Array|MakeArray (Utilities|String|StringToName (Utilities|String|Append "CY" (Utilities|String|ToString(Integer) (Variables|Default|GetYellowCount))))))
              (Math|Integer|IncrementInt (Variables|Default|GetYellowCount))))
          (:then_1
            (if (Math|Vector|NotEqual(Vector) (* (Math|Vector|MakeVector (.Blue_x (Utilities|Struct|BreakDS_Cones _returnvalue)) (.Blue_Y (Utilities|Struct|BreakDS_Cones _returnvalue)) 0.0) _spacing) "0, 0, 0" 0.0001)
              (bind _outhit_2 (Collision|LineTraceByChannel (Math|Vector|MakeVector (.X (Math|Vector|BreakVector (* (Math|Vector|MakeVector (.Blue_x (Utilities|Struct|BreakDS_Cones _returnvalue)) (.Blue_Y (Utilities|Struct|BreakDS_Cones _returnvalue)) 0.0) _spacing))) (.Y (Math|Vector|BreakVector (* (Math|Vector|MakeVector (.Blue_x (Utilities|Struct|BreakDS_Cones _returnvalue)) (.Blue_Y (Utilities|Struct|BreakDS_Cones _returnvalue)) 0.0) _spacing))) 1e+03) (Math|Vector|MakeVector (.X (Math|Vector|BreakVector (* (Math|Vector|MakeVector (.Blue_x (Utilities|Struct|BreakDS_Cones _returnvalue)) (.Blue_Y (Utilities|Struct|BreakDS_Cones _returnvalue)) 0.0) _spacing))) (.Y (Math|Vector|BreakVector (* (Math|Vector|MakeVector (.Blue_x (Utilities|Struct|BreakDS_Cones _returnvalue)) (.Blue_Y (Utilities|Struct|BreakDS_Cones _returnvalue)) 0.0) _spacing))) -1e+03) "TraceTypeQuery1" false 0 "None"))
              (bind _returnvalue_3 (AddComponent|AddChildActorComponent false (Math|Transform|MakeTransform (- (.ImpactPoint (Collision|BreakHitResult _outhit_2)) (Transformation|GetWorldLocation (Variables|Default|GetDefaultSceneRoot))))))
              (ChildActorComponent|SetChildActorClass _returnvalue_3 (Variables|Default|GetBlueCone))
              (Variables|/Script/Engine.Actor|SetTags (Variables|/Script/Engine.ChildActorComponent|GetChildActor _returnvalue_3) (Utilities|Array|MakeArray (Utilities|String|StringToName (Utilities|String|Append "CB" (Utilities|String|ToString(Integer) (Variables|Default|GetBlueCount))))))
              (Math|Integer|IncrementInt (Variables|Default|GetBlueCount)))))))))